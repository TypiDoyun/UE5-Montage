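; Player character with Enhanced Input movement, look, sprint and an automatic-fire weapon that it spawns and attaches to a mesh socket on BeginPlay.
; Sprinting raises walk speed and blocks strafing and backward movement.
; Holding fire loops the Fire montage on completion, decrementing ammo, and plays a Reload montage to refill when empty.
; A separate SpawnProjectile event, not called in this graph, spawns projectiles at the weapon's muzzle.
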(event `self.ReceiveBeginPlay`
  (`|ExecutionSequence`
    (:`then_0`
      (bind `_as플레이어_컨트롤러` (cast `PlayerController` (`self.GetController`)))
      (bind _returnvalue (pcsubsystem `EnhancedInputLocalPlayerSubsystem` `_as플레이어_컨트롤러`))
      (`/Engine/EditorBlueprintResources/StandardMacros.IsValid` _returnvalue
        (:`Is Valid`
          (`EnhancedInputSubsystemInterface.AddMappingContext` _returnvalue "/Game/Input/IMC_YGGroundCharacter.IMC_YGGroundCharacter" 0 (struct)))))
    (:`then_1`
      (bind _returnvalue_2 (`|SpawnActorFromClass` "/Game/YGGame/BP_FPWeapon.BP_FPWeapon_C" (`self.GetTransform`) "AlwaysSpawn" "MultiplyWithRoot" self null))
      (bind _output_get (set `self.CurrentWeapon` _returnvalue_2))
      (`self.K2_AttachToComponent` _output_get (`self.Mesh`) "SocketWeapon" "SnapToTarget" "SnapToTarget" "SnapToTarget" true))
    (:`then_2`
      (set `self.RemainBullets` 10))))

(event `EnhancedInput|/Game/Input/IA_GroundMove`
  (params (ActionValue :type "Vector2D Structure") (ElapsedSeconds :type "Float (double-precision)") (TriggeredSeconds :type "Float (double-precision)") (InputAction :type "InputAction Object Reference" :default "/Game/Input/IA_GroundMove.IA_GroundMove"))
  (bind (_returnvalue_roll _returnvalue_pitch _returnvalue_yaw) (`KismetMathLibrary.BreakRotator` (`self.GetControlRotation`)))
  (bind _returnvalue (`KismetMathLibrary.GetForwardVector` (`KismetMathLibrary.MakeRotator` 0.0 0.0 _returnvalue_yaw)))
  (:`Triggered`
    (`self.AddMovementInput` (`KismetMathLibrary.GetRightVector` (`KismetMathLibrary.MakeRotator` _returnvalue_roll 0.0 _returnvalue_yaw)) (* (`KismetMathLibrary.Conv_BoolToDouble` (not (`self.IsSprinter`))) ActionValue_X))
    (if (`self.IsSprinter`)
      (`self.AddMovementInput` _returnvalue (`KismetMathLibrary.SelectFloat` ActionValue_Y 0.0 (> ActionValue_Y 0.0)))
      (else
        (`self.AddMovementInput` _returnvalue ActionValue_Y)))))

(event `EnhancedInput|/Game/Input/IA_CameraRotate`
  (params (ActionValue :type "Vector2D Structure") (ElapsedSeconds :type "Float (double-precision)") (TriggeredSeconds :type "Float (double-precision)") (InputAction :type "InputAction Object Reference" :default "/Game/Input/IA_CameraRotate.IA_CameraRotate"))
  (:`Triggered`
    (`self.AddControllerYawInput` ActionValue_X)
    (`self.AddControllerPitchInput` ActionValue_Y)))

(event `EnhancedInput|/Game/Input/IA_GroundSprint`
  (params (ActionValue :type Boolean) (ElapsedSeconds :type "Float (double-precision)") (TriggeredSeconds :type "Float (double-precision)") (InputAction :type "InputAction Object Reference" :default "/Game/Input/IA_GroundSprint.IA_GroundSprint"))
  (bind _charactermovement (`self.CharacterMovement`))
  (:`Started`
    (set `self.IsSprinter` true)
    (set `CharacterMovementComponent.MaxWalkSpeed` 600.0 _charactermovement))
  (:`Completed`
    (set `self.IsSprinter` false)
    (set `CharacterMovementComponent.MaxWalkSpeed` 200.0 _charactermovement)))

(event `EnhancedInput|/Game/Input/IA_Fire`
  (params (ActionValue :type Boolean) (ElapsedSeconds :type "Float (double-precision)") (TriggeredSeconds :type "Float (double-precision)") (InputAction :type "InputAction Object Reference" :default "/Game/Input/IA_Fire.IA_Fire"))
  (bind _mesh (`self.Mesh`))
  (:`Started`
    (set `self.IsPushing` true)
    (if (`self.IsPushing`) :!label _label
      (if (> (`self.RemainBullets`) 0)
        (`|PlayMontage` _mesh "/Game/YGGame/MTG_YGCharacterWeaponAction.MTG_YGCharacterWeaponAction" 1.0 0.0 "Fire"
          (:`then`
            (`/Engine/EditorBlueprintResources/StandardMacros.DecrementInt` (`self.RemainBullets`)))
          (:`OnCompleted`
            (goto _label)))
        (elif (not (`self.IsReloading`))
          (`|PlayMontage` _mesh "/Game/YGGame/MTG_YGCharacterWeaponAction.MTG_YGCharacterWeaponAction" 1.0 0.0 "Reload"
            (:`then`
              (set `self.IsReloading` true))
            (:`OnCompleted`
              (set `self.RemainBullets` 10)
              (set `self.IsReloading` false)
              (goto _label)))))))
  (:`Completed`
    (set `self.IsPushing` false)))

(event `SpawnProjectile`
  (bind _currentweapon (`self.CurrentWeapon`))
  (`|SpawnActorFromClass` "/Game/YGGame/BP_YGProjectile.BP_YGProjectile_C" (`SceneComponent.GetSocketTransform` (`/Game/YGGame/BP_FPWeapon.SkeletalMesh` _currentweapon) "Muzzle" "RTS_World") "AlwaysSpawn" "MultiplyWithRoot" _currentweapon self))

(fn `UserConstructionScript`)